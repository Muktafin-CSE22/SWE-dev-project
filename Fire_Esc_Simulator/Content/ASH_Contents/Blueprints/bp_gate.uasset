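; Interactive double gate that the player toggles open and closed with the E key while in range.
; Overlapping the Col component enables input and shows Fr and Fr1; leaving it disables input and hides them.
; An IsOpen flag plays or reverses two timelines, which lerp the yaw of LeftG and RightG to swing the leaves in opposite directions.
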(event OnComponentBeginOverlap(col)
  (params (OverlappedComponent :type Primitive%20Component%20Object%20Reference) (OtherActor :type Actor%20Object%20Reference) (OtherComp :type Primitive%20Component%20Object%20Reference) (OtherBodyIndex :type Integer) (bFromSweep :type Boolean) (SweepResult :type Hit%20Result%20Structure%20%28by%20ref%29))
  (Variables|Default|SetinRange true)
  (Input|EnableInput (Game|GetPlayerController 0))
  (Rendering|SetVisibility (Variables|Default|Getfr) true false)
  (Rendering|SetVisibility (Variables|Default|Getfr1) true false))

(event OnComponentEndOverlap(col)
  (params (OverlappedComponent :type Primitive%20Component%20Object%20Reference) (OtherActor :type Actor%20Object%20Reference) (OtherComp :type Primitive%20Component%20Object%20Reference) (OtherBodyIndex :type Integer))
  (Variables|Default|SetinRange false)
  (Input|DisableInput (Game|GetPlayerController 0))
  (Rendering|SetVisibility (Variables|Default|Getfr) false false)
  (Rendering|SetVisibility (Variables|Default|Getfr1) false false))

(event Input|KeyboardEvents|E
  (params (Key :type Key%20Structure :default "None"))
  (:Pressed
    (if (Variables|Default|GetinRange)
      (if (Variables|Default|GetisOpen)
        (Variables|Default|SetisOpen false)
        (Utilities|FlowControl|Sequence
          (:then_0
            (bind _newtrack_0 (Timeline|Timeline_0 Reverse)
              (:Update
                (Transformation|SetRelativeRotation (Variables|Default|Getleft_g) (Math|Rotator|MakeRotator 0.0 0.0 (Math|Float|Lerp 0.0 -45.0 _newtrack_0)) false false))))
          (:then_1
            (bind _newtrack_0_2 (Timeline|Timeline Reverse)
              (:Update
                (Transformation|SetRelativeRotation (Variables|Default|Getright_g) (Math|Rotator|MakeRotator 0.0 0.0 (Math|Float|Lerp 0.0 45.0 _newtrack_0_2)) false false)))))
        (else
          (Variables|Default|SetisOpen true)
          (Utilities|FlowControl|Sequence
            (:then_0
              (Timeline|Timeline_0 Play))
            (:then_1
              (Timeline|Timeline Play))))))))

(fn ConstructionScript)