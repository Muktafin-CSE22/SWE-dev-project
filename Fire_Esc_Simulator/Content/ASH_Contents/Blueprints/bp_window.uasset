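; Interactive sliding window actor that the player opens and closes with the E key when nearby.
; A box trigger sets an in-range flag, enables input on the actor and shows a text render prompt, undoing all three on exit.
; Each press toggles the open state and plays or reverses a timeline that lerps the window mesh along its relative X axis.
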(event OnComponentBeginOverlap(Box)
  (params (OverlappedComponent :type Primitive%20Component%20Object%20Reference) (OtherActor :type Actor%20Object%20Reference) (OtherComp :type Primitive%20Component%20Object%20Reference) (OtherBodyIndex :type Integer) (bFromSweep :type Boolean) (SweepResult :type Hit%20Result%20Structure%20%28by%20ref%29))
  (Variables|Default|SetinRange true)
  (Input|EnableInput (Game|GetPlayerController 0))
  (Rendering|SetVisibility (Variables|Default|GetTextRender) true false))

(event OnComponentEndOverlap(Box)
  (params (OverlappedComponent :type Primitive%20Component%20Object%20Reference) (OtherActor :type Actor%20Object%20Reference) (OtherComp :type Primitive%20Component%20Object%20Reference) (OtherBodyIndex :type Integer))
  (Variables|Default|SetinRange false)
  (Input|DisableInput (Game|GetPlayerController 0))
  (Rendering|SetVisibility (Variables|Default|GetTextRender) false false))

(event Input|KeyboardEvents|E
  (params (Key :type Key%20Structure :default "None"))
  (:Pressed
    (if (Variables|Default|GetinRange)
      (if (Variables|Default|GetisOpen)
        (Variables|Default|SetisOpen false)
        (bind _winopen (Timeline|Timeline Reverse)
          (:Update
            (Transformation|SetRelativeLocation (Variables|Default|GetSliding_window_003) (Math|Vector|MakeVector (Math|Float|Lerp 0.0 47.0 _winopen) 0.0 0.0) false false)))
        (else
          (Variables|Default|SetisOpen true)
          (Timeline|Timeline Play))))))

(fn ConstructionScript)