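; BP_BigFireDamage is a fire hazard that affects BP_ThirdPersonCharacter through two overlap triggers.
; Trigger sets the character's IsFire flag on entry, clears it on exit, and calls FireDamage both times, leaving damage logic to the character.
; TriggerForCough spawns a 2D cough sound on entry if no valid instance is stored, and stops it on exit.
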(event OnComponentBeginOverlap(Trigger)
  (params (OverlappedComponent :type Primitive%20Component%20Object%20Reference) (OtherActor :type Actor%20Object%20Reference) (OtherComp :type Primitive%20Component%20Object%20Reference) (OtherBodyIndex :type Integer) (bFromSweep :type Boolean) (SweepResult :type Hit%20Result%20Structure%20%28by%20ref%29))
  (bind _asbp_third_person_character (Utilities|Casting|CastToBP_ThirdPersonCharacter OtherActor))
  (Variables|/Game/ThirdPerson/Blueprints/BP_ThirdPersonCharacter.BP_ThirdPersonCharacter_C|SetIsFire _asbp_third_person_character true)
  (Default|FireDamage _asbp_third_person_character))

(event OnComponentEndOverlap(Trigger)
  (params (OverlappedComponent :type Primitive%20Component%20Object%20Reference) (OtherActor :type Actor%20Object%20Reference) (OtherComp :type Primitive%20Component%20Object%20Reference) (OtherBodyIndex :type Integer))
  (bind _asbp_third_person_character (Utilities|Casting|CastToBP_ThirdPersonCharacter OtherActor))
  (Variables|/Game/ThirdPerson/Blueprints/BP_ThirdPersonCharacter.BP_ThirdPersonCharacter_C|SetIsFire _asbp_third_person_character false)
  (Default|FireDamage _asbp_third_person_character))

(event OnComponentBeginOverlap(TriggerForCough)
  (params (OverlappedComponent :type Primitive%20Component%20Object%20Reference) (OtherActor :type Actor%20Object%20Reference) (OtherComp :type Primitive%20Component%20Object%20Reference) (OtherBodyIndex :type Integer) (bFromSweep :type Boolean) (SweepResult :type Hit%20Result%20Structure%20%28by%20ref%29))
  (Utilities|Casting|CastToBP_ThirdPersonCharacter OtherActor)
  (Variables|Default|GetCouchingSound
    (:then)
    (:else
      (bind _returnvalue (Audio|SpawnSound2D "/Game/Sounds/cough-46034.cough-46034" 1.0 1.0 0.0 0))
      (Variables|Default|SetCouchingSound _returnvalue))))

(event OnComponentEndOverlap(TriggerForCough)
  (params (OverlappedComponent :type Primitive%20Component%20Object%20Reference) (OtherActor :type Actor%20Object%20Reference) (OtherComp :type Primitive%20Component%20Object%20Reference) (OtherBodyIndex :type Integer))
  (Utilities|Casting|CastToBP_ThirdPersonCharacter OtherActor)
  (bind _couchingsound (Variables|Default|GetCouchingSound)
    (:then
      (Audio|Components|Audio|Stop _couchingsound))
    (:else)))

(fn ConstructionScript)