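; BP_Fire_Ext is a fire extinguisher pickup that the third-person character can collect.
; Its Box overlap shows either an interact prompt or an "already equipped" notice, depending on whether the character's FireExtingu component is visible, and hides both on exit.
; Interact reveals that component on the player pawn and destroys the pickup if none is equipped, using visibility itself as the equipped state.
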(event OnComponentBeginOverlap(Box)
  (params (OverlappedComponent :type Primitive%20Component%20Object%20Reference) (OtherActor :type Actor%20Object%20Reference) (OtherComp :type Primitive%20Component%20Object%20Reference) (OtherBodyIndex :type Integer) (bFromSweep :type Boolean) (SweepResult :type Hit%20Result%20Structure%20%28by%20ref%29))
  (bind _alreadyequipped (Variables|Default|GetAlreadyEquipped))
  (bind _asbp_third_person_character (Utilities|Casting|CastToBP_ThirdPersonCharacter OtherActor))
  (if (Rendering|IsVisible (Variables|/Game/ThirdPerson/Blueprints/BP_ThirdPersonCharacter.BP_ThirdPersonCharacter_C|GetFire_extingu _asbp_third_person_character))
    (Rendering|SetVisibility _alreadyequipped true false)
    (else
      (Rendering|SetVisibility _alreadyequipped false false)
      (Rendering|SetVisibility (Variables|Default|GetInteract_Widget) true false))))

(event OnComponentEndOverlap(Box)
  (params (OverlappedComponent :type Primitive%20Component%20Object%20Reference) (OtherActor :type Actor%20Object%20Reference) (OtherComp :type Primitive%20Component%20Object%20Reference) (OtherBodyIndex :type Integer))
  (Utilities|Casting|CastToBP_ThirdPersonCharacter OtherActor)
  (Rendering|SetVisibility (Variables|Default|GetInteract_Widget) false false)
  (Rendering|SetVisibility (Variables|Default|GetAlreadyEquipped) false false))

(event EventBeginPlay)

(event Collision|EventActorBeginOverlap
  (params (OtherActor :type Actor%20Object%20Reference)))

(event EventTick
  (params (DeltaSeconds :type Float%20%28single-precision%29)))

(event EventInteract
  (bind _asbp_third_person_character (Utilities|Casting|CastToBP_ThirdPersonCharacter (Game|Player|GetPlayerPawn 0)))
  (if (not (Rendering|IsVisible (Variables|/Game/ThirdPerson/Blueprints/BP_ThirdPersonCharacter.BP_ThirdPersonCharacter_C|GetFire_extingu _asbp_third_person_character)))
    (Rendering|SetVisibility (Variables|/Game/ThirdPerson/Blueprints/BP_ThirdPersonCharacter.BP_ThirdPersonCharacter_C|GetFire_extingu _asbp_third_person_character) true false)
    (Actor|DestroyActor)))

(fn ConstructionScript)

(fn NewFunction)